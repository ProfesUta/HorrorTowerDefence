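; Attack component for BP_FirstPersonCharacter that runs a three-hit sword combo with melee damage.
; Attack input, gated by crouch and CanAttack, plays slash montages by AttackIndex, buffering presses made mid-attack for SwordAttackCombo to continue or reset.
; Input also starts a looping timer that sphere-traces between the sword's two points, damaging "Damageable" actors with a hit sound and short cooldown.
; SwordAttackCombo and StopSwordTrace have no callers in this graph.
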(event `self.ReceiveBeginPlay`
  (bind _asbp_first_person_character (cast `/Game/BP/BP_FirstPersonCharacter` (`self.GetOwner`)))
  (bind _output_get (set `self.CharacterBP` _asbp_first_person_character))
  (set `self.CharacterMesh` (`/Game/BP/BP_FirstPersonCharacter.FirstPersonMesh` _output_get)))

(event `EnhancedInput|/Game/Input/Actions/IA_Attack`
  (params (ActionValue :type Boolean) (ElapsedSeconds :type "Float (double-precision)") (TriggeredSeconds :type "Float (double-precision)") (InputAction :type "InputAction Object Reference" :default "/Game/Input/Actions/IA_Attack.IA_Attack"))
  ; Attack Input
  (:`Started`
    (if (not (`/Game/BP/BP_FirstPersonCharacter.Crouched?` (`self.CharacterBP`)))
      (if (`self.CanAttack?`)
        (`self.SwordAttack`)
        (`self.StartSwordTrace`)))))

(event `Attack1`
  ; Attack 1
  (`/Engine/EditorBlueprintResources/StandardMacros.DoOnce` false :!label _label
    (:`Completed`
      (`KismetSystemLibrary.Delay` 0.1)
      (`|PlayMontage` (`self.CharacterMesh`) "/Game/Characters/Mannequins/Anims/Sword/Sword_Slash_P1_Montage.Sword_Slash_P1_Montage"
        (:`then`
          (set `self.AttackIndex` 1)
          (goto _label :!via `Reset`))))))

(event `SwordAttack`
  ; Sword Attack
  (if (`self.IsAttacking?`)
    (set `self.SaveAttack` true)
    (else
      (set `self.IsAttacking?` true)
      (switch `int` (`self.AttackIndex`) :!label _label_2
        (:`0`
          (`self.Attack1`))
        (:`1`
          (`self.Attack2`))
        (:`2`
          (`self.Attack3`))))))

(event `Attack2`
  ; Attack 2
  (`/Engine/EditorBlueprintResources/StandardMacros.DoOnce` false :!label _label_3
    (:`Completed`
      (`KismetSystemLibrary.Delay` 0.1)
      (`|PlayMontage` (`self.CharacterMesh`) "/Game/Characters/Mannequins/Anims/Sword/Sword_Slash_P2_Montage.Sword_Slash_P2_Montage"
        (:`then`
          (set `self.AttackIndex` 2)
          (goto _label_3 :!via `Reset`))))))

(event `Attack3`
  ; Attack 3
  (`/Engine/EditorBlueprintResources/StandardMacros.DoOnce` false :!label _label_4
    (:`Completed`
      (`KismetSystemLibrary.Delay` 0.1)
      (`|PlayMontage` (`self.CharacterMesh`) "/Game/Characters/Mannequins/Anims/Sword/Sword_Slash_P3_Montage.Sword_Slash_P3_Montage"
        (:`then`
          (set `self.AttackIndex` 3)
          (goto _label_4 :!via `Reset`))))))

(event `SwordAttackCombo`
  ; Combo Continue
  (if (`self.SaveAttack`)
    (set `self.SaveAttack` false)
    (goto _label_2)
    (else
      (`self.StopCombo`))))

(event `StopCombo`
  ; Stop Combo / attack
  (set `self.IsAttacking?` false)
  (set `self.AttackIndex` 0))

(event `StartSwordTrace`
  ; SwordTrace
  (bind _returnvalue (`KismetSystemLibrary.K2_SetTimerDelegate` (delegate `SwordTraceLoop`) 0.1 true))
  (set `self.SwordTraceLoopi` _returnvalue))

(event `PlaySwordHitSound`
  ; SwordHitSound
  (`GameplayStatics.PlaySoundAtLocation` "/Game/Audio/Grunts-Hits/MS_KnifeStab.MS_KnifeStab" (`Actor.K2_GetActorLocation` (`self.GetOwner`)) (struct) 1.0 1.0 0.0 "/Game/Audio/SA_Character.SA_Character" null null null))

(event `SwordTraceLoop`
  (bind _characterbp (`self.CharacterBP`))
  ; SwordTrace
  (bind (_outhit _returnvalue) (`KismetSystemLibrary.SphereTraceSingle` :`Start` (`SceneComponent.K2_GetComponentLocation` (`/Game/BP/BP_FirstPersonCharacter.SwordTopPoint` _characterbp)) :`End` (`SceneComponent.K2_GetComponentLocation` (`/Game/BP/BP_FirstPersonCharacter.SwordBottomPoint` _characterbp)) :`Radius` 12.0 :`TraceChannel` "TraceTypeQuery1" :`DrawTime` 0.1))
  (if _returnvalue
    (bind (_bblockinghit _binitialoverlap _time _distance _location _impactpoint _normal _impactnormal _physmat _hitactor) (`GameplayStatics.BreakHitResult` _outhit))
    (if (`Actor.ActorHasTag` _hitactor "Damageable")
      (`/Engine/EditorBlueprintResources/StandardMacros.DoOnce` false :!label _label_5
        (:`Completed`
          (`GameplayStatics.ApplyDamage` _hitactor (`self.Base Damage`))
          (`self.PlaySwordHitSound`)
          (`KismetSystemLibrary.Delay` 0.5)
          (goto _label_5 :!via `Reset`))))))

(event `StopSwordTrace`
  ; SwordTrace
  (`KismetSystemLibrary.K2_ClearAndInvalidateTimerHandle` (`self.SwordTraceLoopi`)))