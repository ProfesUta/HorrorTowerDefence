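; Stats component shared by the player and zombies, tracking health, plus stamina, XP and level for the player.
; On BeginPlay it waits a tick, casts its owner to set the character type and initializes that owner's HUD.
; Stat functions update widgets directly: health loss selects the player or zombie bar and reports depletion, while other changes target the player HUD.
; Reaching max XP levels up, resetting XP and raising the threshold.
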(event `self.ReceiveBeginPlay`
  (`KismetSystemLibrary.DelayUntilNextTick`)
  (bind _asbp_first_person_character (cast `/Game/BP/BP_FirstPersonCharacter` (`self.GetOwner`))
    (:`then`
      (set `self.PlayerCharacterBP` _asbp_first_person_character)
      (set `self.isPlayer?` true)
      (`ProgressBar.SetPercent` (`/Game/UI/Widgets/WB_HUD.Stamina_Bar` (`/Game/BP/BP_FirstPersonCharacter.HUDWidget` (`self.PlayerCharacterBP`))) (/ (`self.currentStamina`) (`self.maxStamina`)))
      (set `self.characterType` "NewEnumerator0"))
    (:`CastFailed`
      (bind _asbp_zombie (cast `/Game/BP/BP_Zombie` (`self.GetOwner`)))
      (set `self.ZombieAIBP` _asbp_zombie)
      (set `self.isPlayer?` false)
      (set `self.characterType` "NewEnumerator1")))
  (`ProgressBar.SetPercent` (select `/Game/BP/E_CharacterTypes` (`self.characterType`) :`NewEnumerator0` (`/Game/UI/Widgets/WB_HUD.HP_Bar` (`/Game/BP/BP_FirstPersonCharacter.HUDWidget` (`self.PlayerCharacterBP`))) :`NewEnumerator1` (`/Game/UI/Widgets/WB_ZombieHPBar.ZombieHPBar` (`/Game/BP/BP_Zombie.HUDWidget` (`self.ZombieAIBP`)))) (/ (`self.currentHealth`) (`self.maxHealth`)))
  (if (`self.isPlayer?`)
    (`ProgressBar.SetPercent` (`/Game/UI/Widgets/WB_HUD.XP_Bar` (`/Game/BP/BP_FirstPersonCharacter.HUDWidget` (`self.PlayerCharacterBP`))) (/ (`self.XP`) (`self.maxXP`)))
    (`TextBlock.SetText` (`/Game/UI/Widgets/WB_HUD.LVL_Txt` (`/Game/BP/BP_FirstPersonCharacter.HUDWidget` (`self.PlayerCharacterBP`))) (`KismetTextLibrary.Conv_IntToText` (`self.level`)))))

(fn `decreaseHealth`
  (params (DepletedHP :type "Float (double-precision)"))
  (returns (Death :type Boolean))
  (if (not (<= (`self.currentHealth`) 0.0))
    (bind _output_get (set `self.currentHealth` (- (`self.currentHealth`) DepletedHP)))
    (`ProgressBar.SetPercent` (select `/Game/BP/E_CharacterTypes` (`self.characterType`) :`NewEnumerator0` (`/Game/UI/Widgets/WB_HUD.HP_Bar` (`/Game/BP/BP_FirstPersonCharacter.HUDWidget` (`self.PlayerCharacterBP`))) :`NewEnumerator1` (`/Game/UI/Widgets/WB_ZombieHPBar.ZombieHPBar` (`/Game/BP/BP_Zombie.HUDWidget` (`self.ZombieAIBP`)))) (/ _output_get (`self.maxHealth`)))
    (if (<= (`self.currentHealth`) 0.0)
      _
      (else
        (return false))))
  (return true))

(fn `decreaseStamina`
  (params (depletedStamina :type "Float (double-precision)"))
  (returns (noStaminaLeft :type Boolean))
  (if (not (<= (`self.currentStamina`) 0.0))
    (set `self.currentStamina` (- (`self.currentStamina`) depletedStamina))
    (`ProgressBar.SetPercent` (`/Game/UI/Widgets/WB_HUD.Stamina_Bar` (`/Game/BP/BP_FirstPersonCharacter.HUDWidget` (`self.PlayerCharacterBP`))) (/ (`self.currentStamina`) (`self.maxStamina`)))
    (if (<= (`self.maxStamina`) 0.0)
      _
      (else
        (return false))))
  (return true))

(fn `IncreaseHealth`
  (params (AddedHP :type "Float (double-precision)"))
  (set `self.currentHealth` (+ (`self.currentHealth`) AddedHP))
  (if (> (`self.currentHealth`) (`self.maxHealth`))
    (set `self.currentHealth` (`self.maxHealth`)))
  (`ProgressBar.SetPercent` (`/Game/UI/Widgets/WB_HUD.HP_Bar` (`/Game/BP/BP_FirstPersonCharacter.HUDWidget` (`self.PlayerCharacterBP`))) (/ (`self.currentHealth`) (`self.maxHealth`))))

(fn `increaseLVL`
  (params (AddedLVL :type Integer))
  (set `self.level` (+ (`self.level`) AddedLVL))
  (set `self.maxXP` (+ (`self.maxXP`) 150.0))
  (set `self.XP` 0.0)
  (`TextBlock.SetText` (`/Game/UI/Widgets/WB_HUD.LVL_Txt` (`/Game/BP/BP_FirstPersonCharacter.HUDWidget` (`self.PlayerCharacterBP`))) (`KismetTextLibrary.Conv_IntToText` (`self.level`))))

(fn `increaseMaxHealth`
  (params (AddedHP :type "Float (double-precision)"))
  (set `self.maxHealth` (+ (`self.maxHealth`) AddedHP))
  (`ProgressBar.SetPercent` (`/Game/UI/Widgets/WB_HUD.HP_Bar` (`/Game/BP/BP_FirstPersonCharacter.HUDWidget` (`self.PlayerCharacterBP`))) (/ (`self.currentHealth`) (`self.maxHealth`))))

(fn `increaseMaxStamina`
  (params (addedStamina :type "Float (double-precision)"))
  (set `self.maxStamina` (+ (`self.maxStamina`) addedStamina))
  (`ProgressBar.SetPercent` (`/Game/UI/Widgets/WB_HUD.Stamina_Bar` (`/Game/BP/BP_FirstPersonCharacter.HUDWidget` (`self.PlayerCharacterBP`))) (/ (`self.currentStamina`) (`self.maxStamina`))))

(fn `increaseStamina`
  (params (`Added Stamina` :type "Float (double-precision)"))
  (set `self.currentStamina` (+ (`self.currentStamina`) `Added Stamina`))
  (if (> (`self.currentStamina`) (`self.maxStamina`))
    (set `self.currentStamina` (`self.maxStamina`)))
  (`ProgressBar.SetPercent` (`/Game/UI/Widgets/WB_HUD.Stamina_Bar` (`/Game/BP/BP_FirstPersonCharacter.HUDWidget` (`self.PlayerCharacterBP`))) (/ (`self.currentStamina`) (`self.maxStamina`))))

(fn `increaseXP`
  (params (AddedXP :type "Float (double-precision)"))
  (set `self.XP` (+ (`self.XP`) AddedXP))
  (if (>= (`self.XP`) (`self.maxXP`))
    (`self.increaseLVL` 1))
  (`ProgressBar.SetPercent` (`/Game/UI/Widgets/WB_HUD.XP_Bar` (`/Game/BP/BP_FirstPersonCharacter.HUDWidget` (`self.PlayerCharacterBP`))) (/ (`self.XP`) (`self.maxXP`))))